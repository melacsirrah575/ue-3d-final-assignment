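; Game mode for a timed first-person duck shooting gallery, managing the HUD, countdown, target spawning and high score.
; Tick uses one-second Delays to throttle the countdown and spawn three rows of DuckTargets until time runs out, then Reset follows a five-second pause.
; Tick also writes any new high score to a SaveGame slot.
; BeginPlay loads that score and calls Reset only if a save exists.
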(event Custom|SaveHighScore
  ;[1 1 1] Saves highScore
  (if (> (Variables|Default|GetplayersScore) (Variables|Default|GethighScore))
    (Variables|Default|SethighScore (Variables|Default|GetplayersScore))
    (bind _returnvalue (SaveGame|DoesSaveGameExist (Variables|Default|GethighScoreSave)))
    (if _returnvalue
      (bind _returnvalue_2 (SaveGame|LoadGamefromSlot (Variables|Default|GethighScoreSave)))
      (bind _output_get (Variables|Default|SetsaveSubclass _returnvalue_2))
      (bind _assave_game_highscore (Utilities|Casting|CastTosaveGameHighscore _output_get))
      (Variables|/Game/Blueprints/saveGameHighscore.saveGameHighscore_C|SetsavedHighScore _assave_game_highscore (Variables|Default|GethighScore))
      (SaveGame|SaveGametoSlot (Variables|Default|GetsaveSubclass) (Variables|Default|GethighScoreSave))
      (else
        (bind _returnvalue_3 (SaveGame|CreateSaveGameObject "/Game/Blueprints/saveGameHighscore.saveGameHighscore_C"))
        (bind _output_get_2 (Variables|Default|SetsaveSubclass _returnvalue_3))
        (bind _assave_game_highscore_2 (Utilities|Casting|CastTosaveGameHighscore _output_get_2))
        (Variables|/Game/Blueprints/saveGameHighscore.saveGameHighscore_C|SetsavedHighScore _assave_game_highscore_2 (Variables|Default|GethighScore))
        (SaveGame|SaveGametoSlot (Variables|Default|GetsaveSubclass) (Variables|Default|GethighScoreSave))))))

(event Custom|Reset
  (bind _firstpersoncharacter (Variables|Default|GetFirstPersonCharacter))
  ;[1 1 1] Resets Game Variables
  (Variables|Default|SetgameOver false)
  (Variables|Default|SetplayersScore 0)
  (Variables|/Game/Blueprints/PlayerHUD.PlayerHUD_C|SetpointsHUD (Variables|Default|GetPlayerHUD) 0)
  (Variables|Default|SetgameTimeSeconds 0)
  (Variables|Default|SetgameTimeMinutes 2)
  (Variables|/Game/Blueprints/FirstPersonBlueprints/FirstPersonCharacter.FirstPersonCharacter_C|SetcurrentShots _firstpersoncharacter (Variables|/Game/Blueprints/FirstPersonBlueprints/FirstPersonCharacter.FirstPersonCharacter_C|GetmaxShots _firstpersoncharacter)))

(event Custom|SpawnTarget
  ;[1 1 1] Spawn Target
  (Utilities|FlowControl|Delay 1.0)
  ;;[0.9585 1 0] X = Depth, Y = Starting Side, Z = height
  (Game|SpawnActorfromClass "/Game/Blueprints/DuckTarget.DuckTarget_C" (Math|Transform|MakeTransform "-750.000000,500.000000,500.000000" "0, 0, 0" "1,1,1") "Undefined" 0 0) ; Top Row
  (Game|SpawnActorfromClass "/Game/Blueprints/DuckTarget.DuckTarget_C" (Math|Transform|MakeTransform "-900.000000,-700.000000,350.000000" "0.000000,180.000000, 0" "1,1,1") "Undefined" 0 0) ; Middle Row
  (Game|SpawnActorfromClass "/Game/Blueprints/DuckTarget.DuckTarget_C" (Math|Transform|MakeTransform "-1050.000000,500.000000,220.000000" "0, 0, 0" "1,1,1") "Undefined" 0 0) ; Bottom Row
)

(event Custom|GameIsOver
  ;[1 1 1] Game Over
  (Variables|Default|SetgameOver true)
  (Utilities|FlowControl|Delay 5.0)
  (CallFunction|Reset))

(event EventBeginPlay
  ;[1 1 1] Sets HUD
  (bind _returnvalue (UserInterface|CreateWidget "/Game/Blueprints/PlayerHUD.PlayerHUD_C"))
  (bind _output_get (Variables|Default|SetPlayerHUD _returnvalue))
  (UserInterface|Viewport|AddtoViewport _output_get 0)
  ;[1 1 1] Gets FirstPersonCharacter
  (bind _asfirst_person_character (Utilities|Casting|CastToFirstPersonCharacter (Game|GetPlayerCharacter 0)))
  (Variables|Default|SetFirstPersonCharacter _asfirst_person_character)
  ;[1 1 1] Checks for pre-existing and sets highScore
  (bind _returnvalue_2 (SaveGame|DoesSaveGameExist (Variables|Default|GethighScoreSave)))
  (if _returnvalue_2
    (bind _returnvalue_3 (SaveGame|LoadGamefromSlot (Variables|Default|GethighScoreSave)))
    (bind _output_get_2 (Variables|Default|SetsaveSubclass _returnvalue_3))
    (bind _assave_game_highscore (Utilities|Casting|CastTosaveGameHighscore _output_get_2))
    (Variables|Default|SethighScore (Variables|/Game/Blueprints/saveGameHighscore.saveGameHighscore_C|GetsavedHighScore _assave_game_highscore))
    (CallFunction|Reset)))

(event EventTick
  (params (DeltaSeconds :type Float%20%28single-precision%29))
  (if (Variables|Default|GetgameOver)
    _
    (else
      (CallFunction|SpawnTarget)))
  (CallFunction|SaveHighScore)
  ;[1 1 1] Timer Code for PlayerHUD
  (Utilities|FlowControl|Delay 1.0)
  (if (== (Variables|Default|GetgameTimeSeconds) 0)
    (if (== (Variables|Default|GetgameTimeMinutes) 0)
      (CallFunction|GameIsOver)
      (else
        (Variables|Default|SetgameTimeSeconds 59)
        (Math|Integer|DecrementInt (Variables|Default|GetgameTimeMinutes))))
    (else
      (Math|Integer|DecrementInt (Variables|Default|GetgameTimeSeconds)))))

(fn ConstructionScript)

(fn TimerCountdown
  (if (== (Variables|Default|GetgameTimeSeconds) 0)
    (bind _result (Math|Integer|DecrementInt (Variables|Default|GetgameTimeSeconds))
      (:%20%20
        (Development|PrintString (Utilities|String|ToString(Integer) _result))))
    (else
      (Math|Integer|DecrementInt (Variables|Default|GetgameTimeMinutes)
        (:%20%20
          (Variables|Default|SetgameTimeSeconds 60))))))