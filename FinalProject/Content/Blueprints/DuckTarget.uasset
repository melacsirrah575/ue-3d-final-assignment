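; DuckTarget is a moving target actor that travels in a straight line to an end point and then removes itself.
; BeginPlay caches its start location and the world location of its Destination component, so the end point stays fixed while the actor moves.
; Tick advances it at constant MovementSpeed with VInterpToConstant, without sweeping, and destroys it when the remaining distance reaches zero.
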(event EventBeginPlay
  (Variables|Default|SetcurrentLocation (Transformation|GetActorLocation))
  (Variables|Default|SetendPointLocation (Transformation|GetWorldLocation (Variables|Default|GetDestination))))

(event EventTick
  (params (DeltaSeconds :type Float%20%28single-precision%29))
  ;[1 1 1] Movement Logic
  (Variables|Default|SetdeltaTime DeltaSeconds)
  (bind _output_get (Variables|Default|SetcurrentLocation (Math|Interpolation|VInterptoConstant (Variables|Default|GetcurrentLocation) (Variables|Default|GetendPointLocation) (Variables|Default|GetdeltaTime) (Variables|Default|GetmovementSpeed))))
  (Transformation|SetActorLocation _output_get false false)
  (if (<= (Math|Vector|VectorLength (- (Transformation|GetActorLocation) (Variables|Default|GetendPointLocation))) 0.0)
    (Actor|DestroyActor)))

(fn ConstructionScript)