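; MainGameMode is the game mode for a duck target game, handling target spawning, score and the player HUD.
; BeginPlay creates the HUD, then Reset zeroes the score and sets GameTime, which is meant for a timer but never decremented here.
; While GameTime is positive, Tick uses a Delay to spawn DuckTargets at TargetStartingPosition.
; GainPoints adds points, updates the HUD and, as a placeholder, destroys whichever DuckTarget GetActorOfClass returns.
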(event Custom|Gain%20Points
  (params (PointsGained :type Integer))
  ;[1 1 1] Gain Points
  (bind _returnvalue (Actor|GetActorOfClass "/Game/Blueprints/DuckTarget.DuckTarget_C"))
  (Actor|DestroyActor _returnvalue) ; PlaceHolder until Target Animations working
  (bind _output_get (Variables|Default|SetplayersPoints (+ PointsGained (Variables|Default|GetplayersPoints))))
  (Variables|/Game/Blueprints/PlayerHUD.PlayerHUD_C|SetpointsHUD (Variables|Default|GetPlayerHUD) _output_get))

(event Custom|Reset
  ;[1 1 1] Resets Game Variables
  (Variables|Default|SetplayersPoints 0)
  (Variables|/Game/Blueprints/PlayerHUD.PlayerHUD_C|SetpointsHUD (Variables|Default|GetPlayerHUD) 0)
  (Variables|Default|SetgameTime 120) ; Will be used to make a Timer.
)

(event Custom|SpawnTarget
  ;[1 1 1] Spawn Target
  (Game|SpawnActorfromClass "/Game/Blueprints/DuckTarget.DuckTarget_C" (Math|Conversions|ToTransform(Vector) (Variables|Default|GettargetStartingPosition)) "Undefined" 0 0))

(event EventBeginPlay
  ;[1 1 1] Sets HUD
  (bind _returnvalue (UserInterface|CreateWidget "/Game/Blueprints/PlayerHUD.PlayerHUD_C"))
  (bind _output_get (Variables|Default|SetPlayerHUD _returnvalue))
  (UserInterface|Viewport|AddtoViewport _output_get 0)
  (CallFunction|Reset))

(event EventTick
  (params (DeltaSeconds :type Float%20%28single-precision%29))
  ;[1 1 1] Spawns Targets as Long as Game Time != 0
  (if (> (Variables|Default|GetgameTime) 0)
    (Utilities|FlowControl|Delay 1.0)
    (CallFunction|SpawnTarget)))

(fn ConstructionScript)